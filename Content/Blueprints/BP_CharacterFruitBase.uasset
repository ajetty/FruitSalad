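; Base fruit character that gets knocked into a ragdoll when hit by a bulldozer pawn, then recovers.
; A DoOnce-guarded hit disables movement and capsule collision and switches the mesh to physics simulation.
; After a short delay, ReactivateMovement restores walking, moves the capsule to the mesh and snaps the mesh back onto it.
; Random wandering and gradual uprighting logic exist but are disconnected.
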(event Custom|RandomWalker
  (AI|Navigation|SimpleMovetoLocation (Pawn|GetController) (.RandomLocation (AI|Navigation|GetRandomReachablePointinRadius (Transformation|GetActorLocation) 1e+04 0 0))))

(event Custom|ReactivateMovement
  (Utilities|FlowControl|Sequence
    (:then_0
      (Utilities|FlowControl|DoOnce false) ; enters at Reset
    )
    (:then_1
      (Pawn|Components|CharacterMovement|SetMovementMode (Variables|Character|GetCharacterMovement) "MOVE_Walking" 0)
      (Collision|SetCollisionEnabled (Variables|Default|GetCapsuleComponent) "QueryAndPhysics")
      (Collision|SetCollisionEnabled (Variables|Character|GetMesh) "NoCollision")
      (Physics|SetSimulatePhysics (Variables|Character|GetMesh) false)
      (Transformation|SetWorldLocation (Variables|Default|GetCapsuleComponent) (Transformation|GetWorldLocation (Variables|Character|GetMesh)) false false)
      (Transformation|AttachComponentToComponent (Variables|Character|GetMesh) (Variables|Default|GetCapsuleComponent) "None" "SnapToTarget" "SnapToTarget" "SnapToTarget" true))))

(event EventBeginPlay)

(event Collision|EventActorBeginOverlap
  (params (OtherActor :type Actor%20Object%20Reference)))

(event EventTick
  (params (DeltaSeconds :type Float%20%28single-precision%29)))

(event Collision|EventHit
  (params (MyComp :type Primitive%20Component%20Object%20Reference) (Other :type Actor%20Object%20Reference) (OtherComp :type Primitive%20Component%20Object%20Reference) (bSelfMoved :type Boolean) (HitLocation :type Vector :default "0, 0, 0") (HitNormal :type Vector :default "0, 0, 0") (NormalImpulse :type Vector :default "0, 0, 0") (Hit :type Hit%20Result%20Structure%20%28by%20ref%29))
  (Utilities|Casting|CastToPawnBulldozer (Components|GetOwner OtherComp))
  (Utilities|FlowControl|DoOnce false
    (:Completed
      (Pawn|Components|CharacterMovement|DisableMovement (Variables|Character|GetCharacterMovement))
      (Collision|SetCollisionEnabled (Variables|Default|GetCapsuleComponent) "NoCollision")
      (Collision|SetCollisionEnabled (Variables|Character|GetMesh) "QueryAndPhysics")
      (Physics|SetSimulatePhysics (Variables|Character|GetMesh) true)
      (Utilities|FlowControl|Delay 3.0)
      (CallFunction|ReactivateMovement))))

(fn ConstructionScript)